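; Entity is an RTS actor that spawns units in response to a debug-style key press.
; Pressing 0 prints a message, then clears CurrentUnit if the first slot of the Units array holds a valid unit.
; Otherwise it spawns a Unit at its own transform and inserts it at the front of the array.
; The default BeginPlay, overlap and Tick events are disabled, and the construction script only calls its parent.
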(event EventBeginPlay
  (|CallParentFunction) ; This node is disabled and will not be called.\nDrag off pins to build functionality.
)

(event Collision|EventActorBeginOverlap
  (params (OtherActor :type Actor%20Object%20Reference)))

(event EventTick
  (params (DeltaSeconds :type Float%20%28single-precision%29)))

(event Input|KeyboardEvents|0
  (params (Key :type Key%20Structure :default "None"))
  (:Pressed
    (Development|PrintString "Button 0 pressed")
    (if (Utilities|IsValid (Utilities|Array|Get(acopy) (Variables|Default|GetUnits)))
      (Variables|Default|SetCurrentUnit 0)
      (else
        (bind _returnvalue (Game|SpawnActorfromClass "/Game/NaniteRTS/Blueprints/Unit.Unit_C" (Transformation|GetActorTransform) "Undefined" "MultiplyWithRoot" 0 0))
        (Utilities|Array|Insert (Variables|Default|GetUnits) _returnvalue)))))

(fn ConstructionScript
  (|CallParentFunction))