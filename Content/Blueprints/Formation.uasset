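; Formation actor that spawns units in a hollow square when play begins.
; BeginPlay passes the unit count, start and end positions and spacing to HollowSquareFormation with a fixed wall thickness.
; It force-spawns a Unit at each returned position regardless of collision, then prints the count.
; A disconnected SquareFormation branch with a debug print remains as an unused alternative into the same spawn loop.
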(event EventBeginPlay
  (bind _returnvalue (Class|Formation|HollowSquareFormation (Variables|Default|GetnbUnits) (Variables|Default|GetStart%20Pos) (Variables|Default|GetEnd%20Pos) (Variables|Default|Getspacing) 3))
  (for _array_element _returnvalue
    (Game|SpawnActorfromClass "/Game/Blueprints/Unit.Unit_C" (Math|Conversions|ToTransform(Vector) _array_element) "AlwaysSpawn" "MultiplyWithRoot" 0 0))
  (Development|PrintString (Utilities|String|Append "Instantiated " (Utilities|String|ToString(Integer) (Utilities|Array|Length _returnvalue)) " units")))

(event Collision|EventActorBeginOverlap
  (params (OtherActor :type Actor%20Object%20Reference)))

(event EventTick
  (params (DeltaSeconds :type Float%20%28single-precision%29)))

(fn ConstructionScript)